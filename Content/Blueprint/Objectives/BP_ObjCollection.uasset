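; Objective that groups a collection of child objectives and counts as complete only when every child is complete.
; On activation it either activates all children at once or, when OrderRequired is set, only the first incomplete one.
; In ordered mode it binds to that child's OnCompleted, then unbinds and activates the next incomplete child, chaining them in sequence.
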(event Custom|OnCompleted_Event_0
  (params (Objective :type BP%20Objective%20Object%20Reference))
  (EventDispatchers|UnbindEventfromOnCompleted Objective (delegate Custom|OnCompleted_Event_0))
  (bind _nextobjective (Private|FindNextIncompleteObject))
  (Utilities|IsValid _nextobjective
    (:Is%20Valid
      (Default|ActivateObjective _nextobjective)
      (EventDispatchers|AssignOnCompleted _nextobjective (delegate Custom|OnCompleted_Event_0)))))

(event EventActivateObjective
  (|CallParentFunction)
  (if (Variables|Default|GetOrderRequired)
    (bind _nextobjective (Private|FindNextIncompleteObject))
    (Utilities|IsValid _nextobjective
      (:Is%20Valid
        (Default|ActivateObjective _nextobjective)
        (EventDispatchers|AssignOnCompleted _nextobjective (delegate Custom|OnCompleted_Event_0))))
    (else
      (for _array_element (Variables|Public|GetObjectives)
        (Default|ActivateObjective _array_element)))))

(fn FindNextIncompleteObject
  (for _array_element (Variables|Public|GetObjectives)
    (if (not (CallFunction|GetIsComplete _array_element))
      (return _array_element)))
  (return 0))

(fn AddObjectives
  (params (Objective :type BP%20Objective%20Object%20Reference%20%28by%20ref%29))
  (Utilities|Array|Add (Variables|Public|GetObjectives) Objective))

(fn GetIsComplete
  (for _array_element (Variables|Public|GetObjectives)
    (if (not (CallFunction|GetIsComplete _array_element))
      (return false)))
  (return true))