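; An objective that completes when the player character reaches a destination actor.
; On activation it binds to the destination's begin-overlap event and ignores anything that is not the third-person character.
; On the first valid overlap it unbinds, sets a reached flag that GetIsComplete reports, and fires the completion event.
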(event Custom|OnActorBeginOverlap_Event_0
  (params (OverlappedActor :type Actor%20Object%20Reference) (OtherActor :type Actor%20Object%20Reference))
  (Utilities|Casting|CastToBP_ThirdPersonCharacter OtherActor)
  (Collision|UnbindEventfromOnActorBeginOverlap (Variables|Default|GetDestination) (delegate Custom|OnActorBeginOverlap_Event_0))
  (Variables|Default|SetReachedDestination true)
  (Default|CallOnCompleted self))

(event EventActivateObjective
  (|CallParentFunction)
  (EventDispatchers|AssignOnActorBeginOverlap (Variables|Default|GetDestination) (delegate Custom|OnActorBeginOverlap_Event_0)))

(fn GetIsComplete
  (return (Variables|Default|GetReachedDestination)))