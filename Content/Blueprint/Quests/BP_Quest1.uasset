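; BP_Quest1 defines the "A long Way Home" quest, in which the player travels to three cities in order.
; ConstructRootObjCollection creates the root objective collection with ordering required.
; PopulateObjectives then builds a reach-destination objective for each city's trigger and adds it to that collection in sequence.
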(fn ConstructionScript
  (|CallParentFunction))

(fn ConstructRootObjCollection
  (bind _returnvalue (Game|ConstructObjectfromClass self "/Game/Blueprint/Objectives/BP_ObjCollection.BP_ObjCollection_C" true "A long Way Home"))
  (return _returnvalue))

(fn PopulateObjectives
  (params (RootObjCollection :type BP%20Obj%20Collection%20Object%20Reference))
  (Utilities|FlowControl|Sequence
    (:then_0
      (bind _returnvalue (Game|ConstructObjectfromClass self "/Game/Blueprint/Objectives/BP_ObjReachDestination.BP_ObjReachDestination_C" (Variables|Default|GetCity1Trigger) "Reeach City1"))
      (Default|AddObjectives RootObjCollection _returnvalue))
    (:then_1
      (bind _returnvalue_2 (Game|ConstructObjectfromClass self "/Game/Blueprint/Objectives/BP_ObjReachDestination.BP_ObjReachDestination_C" (Variables|Default|GetCity2Trigger) "Reeach City2"))
      (Default|AddObjectives RootObjCollection _returnvalue_2))
    (:then_2
      (bind _returnvalue_3 (Game|ConstructObjectfromClass self "/Game/Blueprint/Objectives/BP_ObjReachDestination.BP_ObjReachDestination_C" (Variables|Default|GetCity3Trigger) "Reeach City3"))
      (Default|AddObjectives RootObjCollection _returnvalue_3))))