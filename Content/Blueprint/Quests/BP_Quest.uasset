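; BP_Quest is a base Blueprint for quests, holding a root objective collection that other code reads through a getter.
; On BeginPlay it constructs and stores the root collection, then passes it to PopulateObjectives.
; Both the construct and populate functions are placeholders that only print red error messages, so child quest Blueprints are expected to override them in a template-method pattern.
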(event EventBeginPlay
  (bind _rootobjcollection (Private|ConstructRootObjCollection))
  (bind _output_get (Variables|Private|SetRootObjectiveCollection _rootobjcollection))
  (Private|PopulateObjectives _output_get))

(fn ConstructionScript)

(fn ConstructRootObjCollection
  (Development|PrintString "Error:  Create RootObjectiveCollection called for base class" true true "(R=0.475000,G=0.000000,B=0.031700,A=1.000000)")
  (return 0))

(fn PopulateObjectives
  (params (RootObjCollection :type BP%20Obj%20Collection%20Object%20Reference))
  (Development|PrintString "Error: PopulateObjectiveCollection called for base class" true true "(R=0.475000,G=0.000000,B=0.031700,A=1.000000)")
  (return))

(fn GetRootObjectiveCollection
  (return (Variables|Private|GetRootObjectiveCollection)))