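; BP_Light is an interactable light that the player can switch on and off with the F key.
; A Sphere overlap with BP_ThirdPersonCharacter enables input on the actor for that character's controller, and leaving the sphere disables it.
; Pressing F toggles the PointLight's visibility, and an IsON? function reports whether it is currently visible.
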(event OnComponentBeginOverlap(Sphere)
  (params (OverlappedComponent :type Primitive%20Component%20Object%20Reference) (OtherActor :type Actor%20Object%20Reference) (OtherComp :type Primitive%20Component%20Object%20Reference) (OtherBodyIndex :type Integer) (bFromSweep :type Boolean) (SweepResult :type Hit%20Result%20Structure%20%28by%20ref%29))
  (bind _asbp_third_person_character (Utilities|Casting|CastToBP_ThirdPersonCharacter OtherActor))
  (Input|EnableInput (.AsPlayer%20Controller (Utilities|Casting|CastToPlayerController (Pawn|GetController _asbp_third_person_character)))))

(event OnComponentEndOverlap(Sphere)
  (params (OverlappedComponent :type Primitive%20Component%20Object%20Reference) (OtherActor :type Actor%20Object%20Reference) (OtherComp :type Primitive%20Component%20Object%20Reference) (OtherBodyIndex :type Integer))
  (bind _asbp_third_person_character (Utilities|Casting|CastToBP_ThirdPersonCharacter OtherActor))
  (Input|DisableInput (.AsPlayer%20Controller (Utilities|Casting|CastToPlayerController (Pawn|GetController _asbp_third_person_character)))))

(event Input|KeyboardEvents|F
  (params (Key :type Key%20Structure :default "None"))
  (:Pressed
    (Rendering|ToggleVisibility (Variables|Default|GetPointLight) false)))

(fn ConstructionScript)

(fn IsON?
  (return (Variables|/Script/Engine.SceneComponent|GetbVisible (Variables|Default|GetPointLight))))